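; BP_RewindActor is a test actor that records a physics-simulated cube's movement and rewinds it after a short delay.
; On BeginPlay, Record enables physics on the Cube and starts recording through a RewindTime component.
; After the delay, Rewind starts the component's rewind playback and turns physics off so the recorded motion drives the cube.
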(event Custom|Record
  (Physics|SetSimulatePhysics (Variables|Default|GetCube) true)
  (Class|RewindTimeComponent|StartRecordMovement (Variables|Default|GetRewindTime)))

(event Custom|Rewind
  (Class|RewindTimeComponent|StartRewindMovement (Variables|Default|GetRewindTime))
  (Physics|SetSimulatePhysics (Variables|Default|GetCube) false))

(event EventBeginPlay
  (CallFunction|Record)
  (Utilities|FlowControl|Delay 5.0)
  (CallFunction|Rewind))

(fn ConstructionScript)